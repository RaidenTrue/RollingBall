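; Floor button that latches when a BP_BallPawn overlaps its sphere, playing a sound and turning green.
; On press it calls OnPickup on linked AffectedActors (other buttons or BP_LaunchActors), and each such match plays the Z-offset timeline.
; A button's own OnPickup resets it to orange, unlatches it and reverses the timeline, so buttons can release one another.
; A dynamic material instance created at construction drives the color.
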(event OnComponentBeginOverlap(OverlapSphere)
  (params (OverlappedComponent :type Primitive%20Component%20Object%20Reference) (OtherActor :type Actor%20Object%20Reference) (OtherComp :type Primitive%20Component%20Object%20Reference) (OtherBodyIndex :type Integer) (bFromSweep :type Boolean) (SweepResult :type Hit%20Result%20Structure%20%28by%20ref%29))
  (bind _initialbuttonlocation (Variables|Default|GetInitialButtonLocation))
  (bind (_x _y _z) (Math|Vector|BreakVector _initialbuttonlocation))
  (Utilities|Casting|CastToBP_BallPawn OtherActor)
  ;[1 1 1] CheckIfButtonIsPressed
  (if (not (Variables|Default|GetButtonPressed))
    (Variables|Default|SetButtonPressed true)
    (Audio|PlaySound2D "/Game/Retro_8Bit_Sounds/Collectables/Cues/retro_collect_pickup_item_08_Cue.retro_collect_pickup_item_08_Cue" 1.0 1.0 0.0 0 0)
    ;[1 1 1] ChangeColorWhenPressed
    (Rendering|Material|SetVectorParameterValue (Variables|Default|GetOrangeMaterialInst) "Color" "(R=0.062544,G=0.687500,B=0.018105,A=1.000000)" :!class /Script/Engine.MaterialInstanceDynamic)
    (for _array_element (Variables|Default|GetAffectedActors)
      (bind _asbp_button (Utilities|Casting|CastToBP_Button _array_element)
        (:then
          (Default|OnPickup _asbp_button)
          (bind _buttonelevation (Timeline|ButtonTimeline Play)
            (:Update
              (Transformation|SetWorldLocation (Variables|Default|GetButton) (Math|Vector|MakeVector _x _y (+ _z _buttonelevation)) false false))))
        (:CastFailed
          (bind _asbp_launch_actor (Utilities|Casting|CastToBP_LaunchActor _array_element))
          (Default|OnPickup _asbp_launch_actor)
          (Timeline|ButtonTimeline Play))))))

(event OnComponentEndOverlap(OverlapSphere)
  (params (OverlappedComponent :type Primitive%20Component%20Object%20Reference) (OtherActor :type Actor%20Object%20Reference) (OtherComp :type Primitive%20Component%20Object%20Reference) (OtherBodyIndex :type Integer))
  ;[1 1 1] NotUsing
  (Utilities|Casting|CastToBP_BallPawn OtherActor))

(event EventBeginPlay
  ;[1 1 1] GetButtonWorldLocation
  (Variables|Default|SetInitialButtonLocation (Transformation|GetWorldLocation (Variables|Default|GetButton))))

(event Collision|EventActorBeginOverlap
  (params (OtherActor :type Actor%20Object%20Reference)))

(event EventTick
  (params (DeltaSeconds :type Float%20%28single-precision%29)))

(event EventOnPickup
  (bind _initialbuttonlocation (Variables|Default|GetInitialButtonLocation))
  (bind (_x _y _z) (Math|Vector|BreakVector _initialbuttonlocation))
  (Rendering|Material|SetVectorParameterValue (Variables|Default|GetOrangeMaterialInst) "Color" "(R=0.800000,G=0.300000,B=0.000000,A=1.000000)" :!class /Script/Engine.MaterialInstanceDynamic)
  (Variables|Default|SetButtonPressed false)
  (bind _buttonelevation (Timeline|ButtonTimeline Reverse)
    (:Update
      (Transformation|SetWorldLocation (Variables|Default|GetButton) (Math|Vector|MakeVector _x _y (+ _z _buttonelevation)) false false))))

(fn ConstructionScript
  (bind _returnvalue (Rendering|Material|CreateDynamicMaterialInstance "/Game/Blueprints/Materials/MI_Orange_Shiny.MI_Orange_Shiny" "None" "None" :!class /Script/Engine.KismetMaterialLibrary))
  (bind _output_get (Variables|Default|SetOrangeMaterialInst _returnvalue))
  (Rendering|Material|SetMaterial (Variables|Default|GetButton) 0 _output_get))