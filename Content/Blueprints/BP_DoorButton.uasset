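; A pressure button actor that moves a linked door while a BP_BallPawn rests inside its sphere trigger.
; Overlap begin plays a sound and runs ButtonTimeline forward; overlap end reverses it from its current position.
; Each timeline update feeds button and door elevation tracks into UpdateVectors, which offsets both components' world Z from locations cached at BeginPlay.
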(event OnComponentBeginOverlap(Sphere)
  (params (OverlappedComponent :type Primitive%20Component%20Object%20Reference) (OtherActor :type Actor%20Object%20Reference) (OtherComp :type Primitive%20Component%20Object%20Reference) (OtherBodyIndex :type Integer) (bFromSweep :type Boolean) (SweepResult :type Hit%20Result%20Structure%20%28by%20ref%29))
  (Utilities|Casting|CastToBP_BallPawn OtherActor)
  (Audio|PlaySound2D "/Game/Retro_8Bit_Sounds/Collectables/Wavs/retro_collect_pickup_item_08.retro_collect_pickup_item_08" 1.0 1.0 0.0 0 0)
  (bind (_direction _buttonelevation _doorelevation) (Timeline|ButtonTimeline Play)
    (:Update
      (CallFunction|UpdateVectors _buttonelevation _doorelevation))))

(event OnComponentEndOverlap(Sphere)
  (params (OverlappedComponent :type Primitive%20Component%20Object%20Reference) (OtherActor :type Actor%20Object%20Reference) (OtherComp :type Primitive%20Component%20Object%20Reference) (OtherBodyIndex :type Integer))
  (Utilities|Casting|CastToBP_BallPawn OtherActor)
  (bind (_direction _buttonelevation _doorelevation) (Timeline|ButtonTimeline Reverse)
    (:Update
      (CallFunction|UpdateVectors _buttonelevation _doorelevation))))

(event EventBeginPlay
  (Variables|Default|SetInitialButtonLocation (Transformation|GetWorldLocation (Variables|Default|GetButton)))
  (Variables|Default|SetInitialDoorLocation (Transformation|GetWorldLocation (Variables|Default|GetDoor))))

(event Collision|EventActorBeginOverlap
  (params (OtherActor :type Actor%20Object%20Reference)))

(event EventTick
  (params (DeltaSeconds :type Float%20%28single-precision%29)))

(event Collision|EventHit
  (params (MyComp :type Primitive%20Component%20Object%20Reference) (Other :type Actor%20Object%20Reference) (OtherComp :type Primitive%20Component%20Object%20Reference) (bSelfMoved :type Boolean) (HitLocation :type Vector :default "0, 0, 0") (HitNormal :type Vector :default "0, 0, 0") (NormalImpulse :type Vector :default "0, 0, 0") (Hit :type Hit%20Result%20Structure%20%28by%20ref%29)))

(fn ConstructionScript)

(fn UpdateVectors
  (params (ButtonElevation :type Float%20%28single-precision%29) (DoorElevation :type Float%20%28single-precision%29))
  (bind _initialbuttonlocation (Variables|Default|GetInitialButtonLocation))
  (bind _initialdoorlocation (Variables|Default|GetInitialDoorLocation))
  (bind (_x _y _z) (Math|Vector|BreakVector _initialdoorlocation))
  (bind (_x_2 _y_2 _z_2) (Math|Vector|BreakVector _initialbuttonlocation))
  (Utilities|FlowControl|Sequence
    (:then_0
      ;[1 1 1] SetButtonLocation
      (Transformation|SetWorldLocation (Variables|Default|GetButton) (Math|Vector|MakeVector _x_2 _y_2 (+ _z_2 ButtonElevation)) false false))
    (:then_1
      ;[1 1 1] SetDoorLocation
      (Transformation|SetWorldLocation (Variables|Default|GetDoor) (Math|Vector|MakeVector _x _y (+ _z DoorElevation)) false false))))