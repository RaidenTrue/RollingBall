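; Player pawn for a rolling-ball pickup game, handling movement, camera, jumping, score and health.
; Input applies camera-relative torque to the physics mesh; jump adds an impulse, re-armed by hits on a custom collision channel.
; BeginPlay counts pickups, excluding explosives and health, as goal targets; collecting them all calls CallDestroyHazards.
; Zero health only prints a message, and heals reaching MaxHealth are ignored rather than clamped.
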(event EventBeginPlay
  (bind _outactors (Actor|GetAllActorsOfClass "/Game/Blueprints/Pickup/BP_PickupBase.BP_PickupBase_C"))
  (for _array_element _outactors
    (Utilities|Casting|CastToBP_Explosive _array_element
      (:CastFailed
        (Utilities|Casting|CastToBP_HealthPickup _array_element
          (:CastFailed
            (bind _output_get (Variables|Default|SetTotalGoalTargets (+ (Variables|Default|GetTotalGoalTargets) 1))))))))
  (Development|PrintString (Utilities|String|ToString(Integer) _output_get)))

(event Collision|EventActorBeginOverlap
  (params (OtherActor :type Actor%20Object%20Reference)))

(event EventTick
  (params (DeltaSeconds :type Float%20%28single-precision%29)))

(event Collision|EventHit
  (params (MyComp :type Primitive%20Component%20Object%20Reference) (Other :type Actor%20Object%20Reference) (OtherComp :type Primitive%20Component%20Object%20Reference) (bSelfMoved :type Boolean) (HitLocation :type Vector :default "0, 0, 0") (HitNormal :type Vector :default "0, 0, 0") (NormalImpulse :type Vector :default "0, 0, 0") (Hit :type Hit%20Result%20Structure%20%28by%20ref%29))
  ;[1 1 1] Jump & CanJump Condition
  (if (Utilities|Enum|Equal(Enum) (Collision|GetCollisionObjectType OtherComp) "ECC_GameTraceChannel1")
    (if (Variables|Default|GetCanJump)
      _
      (else
        (Audio|PlaySound2D "/Game/Retro_8Bit_Sounds/Impacts/Cues/retro_impact_hit_11_Cue.retro_impact_hit_11_Cue" 1.0 1.0 0.0 0 0)))
    (Variables|Default|SetCanJump true)))

(event Input|ActionEvents|InputActionJump
  (params (Key :type Key%20Structure :default "None"))
  ;[1 1 1] Jump & CanJump Condition
  (:Pressed
    (if (Variables|Default|GetCanJump)
      (Physics|AddImpulse (Variables|Default|GetBallMesh) (Math|Vector|MakeVector 0.0 0.0 (* (Variables|Default|GetJump) 1.0)) "None" true)
      (Variables|Default|SetCanJump false)
      (Audio|PlaySound2D "/Game/Retro_8Bit_Sounds/Jumping/Cues/retro_jump_bounce_12_Cue.retro_jump_bounce_12_Cue" 1.0 1.0 0.0 0 0))))

(event Input|AxisEvents|InputAxisMoveForward/Backward
  (params (AxisValue :type Float%20%28single-precision%29))
  ;[1 1 1] MoveForward/Backward
  (Class|PrimitiveComponent|AddTorqueinDegrees (Variables|Default|GetBallMesh) (* (* (Math|Vector|GetRightVector (Pawn|GetControlRotation :!class /Script/Engine.Pawn)) (Variables|Default|GetTorque)) AxisValue) "None" true))

(event Input|AxisEvents|InputAxisMoveRight/Left
  (params (AxisValue :type Float%20%28single-precision%29))
  ;[1 1 1] Move Right/Left
  (Class|PrimitiveComponent|AddTorqueinDegrees (Variables|Default|GetBallMesh) (* (Math|Vector|GetForwardVector (Math|Rotator|MakeRotator 0.0 0.0 (.Yaw (Math|Rotator|BreakRotator (Pawn|GetControlRotation :!class /Script/Engine.Pawn))))) (* (Variables|Default|GetTorque) AxisValue -1.0)) "None" true))

(event Input|AxisEvents|InputAxisLookUp
  (params (AxisValue :type Float%20%28single-precision%29))
  ;[1 1 1] MouseCameraControls
  (Pawn|Input|AddControllerPitchInput (* AxisValue -1.0)))

(event Input|AxisEvents|InputAxisTurn
  (params (AxisValue :type Float%20%28single-precision%29))
  ;[1 1 1] MouseCameraControls
  (Pawn|Input|AddControllerYawInput AxisValue))

(event Input|AxisEvents|InputAxisLookUpRate
  (params (AxisValue :type Float%20%28single-precision%29))
  ;[1 1 1] Up&Down ArrowKeyInput
  (Pawn|Input|AddControllerPitchInput (* AxisValue (Variables|Default|GetTurnRate) (Utilities|Time|GetWorldDeltaSeconds))))

(event Input|AxisEvents|InputAxisTurnRate
  (params (AxisValue :type Float%20%28single-precision%29))
  ;[1 1 1] Right&Left ArrowKeyInput
  (Pawn|Input|AddControllerYawInput (* AxisValue (Variables|Default|GetLookUpRate) (Utilities|Time|GetWorldDeltaSeconds))))

(event Input|KeyboardEvents|Escape
  (params (Key :type Key%20Structure :default "None"))
  ;[1 1 1] QuitGame
  (:Pressed
    (Game|QuitGame 0 "Quit" false)))

(fn ConstructionScript)

(fn ScoreIncrement
  (params (InScore :type Integer))
  (Variables|Default|SetScore (+ (Variables|Default|GetScore) InScore)))

(fn IncrementGoalTargets
  (Variables|Default|SetGoalTargets (+ (Variables|Default|GetGoalTargets) 1))
  (if (== (Variables|Default|GetGoalTargets) (Variables|Default|GetTotalGoalTargets))
    (Default|CallDestroyHazards)))

(fn DecrementHealth
  (params (Amount :type Float%20%28single-precision%29))
  (if (<= (- (Variables|Default|GetHealth) Amount) 0.0)
    (Development|PrintString "HEALTH ZERO!!!!")
    (else
      (Variables|Default|SetHealth (- (Variables|Default|GetHealth) Amount)))))

(fn IncrementHealth
  (params (Amount :type Float%20%28single-precision%29))
  (if (not (>= (+ Amount (Variables|Default|GetHealth)) (Variables|Default|GetMaxHealth)))
    (Variables|Default|SetHealth (+ Amount (Variables|Default|GetHealth)))))