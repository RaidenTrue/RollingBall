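; BP_Explosive is an explosive hazard pickup that damages and launches the player's ball when picked up.
; On pickup it decrements ball health, applies a radial impulse from below its origin and silences its looping sparks sound before calling parent logic.
; BeginPlay configures inherited pickup settings for zero points and explosion effects, starts the sound, and binds DestroySelf to the player's destroy-hazards event, which sparkles before removing the actor.
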(event Custom|DestroySelf
  (Effects|SpawnEmitteratLocation "/Game/InfinityBladeEffects/Effects/FX_Treasure/Gold_Bag/P_GoldSparkle_Bag_Lo_2.P_GoldSparkle_Bag_Lo_2" (Transformation|GetActorLocation))
  (Utilities|FlowControl|Delay 0.5)
  (Actor|DestroyActor))

(event EventBeginPlay
  (Variables|Default|SetUseNumberWidget false)
  (Variables|Default|SetPoints 0)
  (Variables|Default|SetCoinPickup "/Game/StarterContent/Audio/Explosion01.Explosion01")
  (Variables|Default|SetOnPickupParticles "/Game/StarterContent/Particles/P_Explosion.P_Explosion")
  (bind _returnvalue (Audio|SpawnSoundatLocation "/Game/StarterContent/Audio/Fire_Sparks01_Cue.Fire_Sparks01_Cue" (Transformation|GetActorLocation) "0, 0, 0" 1.0 1.0 0.0 0 0))
  (Variables|Default|SetSparksSound _returnvalue)
  (|CallParentFunction)
  (EventDispatchers|BindEventtoDestroyHazards (.AsBP%20Ball%20Pawn (Utilities|Casting|CastToBP_BallPawn (Game|Player|GetPlayerPawn 0))) (delegate Custom|DestroySelf)))

(event Collision|EventActorBeginOverlap
  (params (OtherActor :type Actor%20Object%20Reference))
  (|CallParentFunction OtherActor) ; This node is disabled and will not be called.\nDrag off pins to build functionality.
)

(event EventTick
  (params (DeltaSeconds :type Float%20%28single-precision%29))
  (|CallParentFunction DeltaSeconds) ; This node is disabled and will not be called.\nDrag off pins to build functionality.
)

(event EventOnPickup
  (params (OtherActor :type Object%20Object%20Reference))
  (bind _returnvalue (Transformation|GetActorLocation))
  (bind (_x _y _z) (Math|Vector|BreakVector _returnvalue))
  ;[1 1 1] OnPickup Explodes
  (bind _asbp_ball_pawn (Utilities|Casting|CastToBP_BallPawn OtherActor))
  (Default|DecrementHealth _asbp_ball_pawn (Variables|Default|GetDamage))
  (Physics|AddRadialImpulse (Variables|/Game/Blueprints/BP_BallPawn.BP_BallPawn_C|GetBallMesh _asbp_ball_pawn) (Math|Vector|MakeVector _x _y (+ _z -75.0)) 5e+02 1e+03 "RIF_Constant" true)
  (Components|Activation|SetActive (Variables|Default|GetSparksSound) false false)
  (|CallParentFunction OtherActor))

(fn ConstructionScript
  (|CallParentFunction))