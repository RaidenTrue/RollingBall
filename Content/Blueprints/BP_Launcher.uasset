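; BP_Launcher is a launcher button that flings a BP_BallPawn along the button's up vector when the ball hits it.
; The hit applies a velocity-change impulse to the ball mesh, plays a 2D sound and starts a timeline.
; The timeline offsets the button's Z from the location cached at BeginPlay, and a short Delay fired from its Update then reverses it.
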(event OnComponentHit(Button)
  (params (HitComponent :type Primitive%20Component%20Object%20Reference) (OtherActor :type Actor%20Object%20Reference) (OtherComp :type Primitive%20Component%20Object%20Reference) (NormalImpulse :type Vector :default "0, 0, 0") (Hit :type Hit%20Result%20Structure%20%28by%20ref%29))
  (bind _initialbuttonlocation (Variables|Default|GetInitialButtonLocation))
  (bind (_x _y _z) (Math|Vector|BreakVector _initialbuttonlocation))
  (bind _asbp_ball_pawn (Utilities|Casting|CastToBP_BallPawn OtherActor))
  (Physics|AddImpulse (Variables|/Game/Blueprints/BP_BallPawn.BP_BallPawn_C|GetBallMesh _asbp_ball_pawn) (* (Math|Vector|GetUpVector (Variables|Default|GetButton)) (Variables|Default|GetImpulse)) "None" true)
  (Audio|PlaySound2D "/Game/Retro_8Bit_Sounds/Damage_Hurt/Cues/retro_damage_hurt_ouch_01_Cue.retro_damage_hurt_ouch_01_Cue" 1.0 1.0 0.0 0 0)
  (bind _launchelevation (Timeline|Launcher_Timeline Play)
    (:Update
      (Transformation|SetWorldLocation (Variables|Default|GetButton) (Math|Vector|MakeVector _x _y (+ _launchelevation _z)) false false)
      (Utilities|FlowControl|Delay 0.2)
      (Timeline|Launcher_Timeline Reverse))))

(event EventBeginPlay
  (Variables|Default|SetInitialButtonLocation (Transformation|GetWorldLocation (Variables|Default|GetButton))))

(event Collision|EventActorBeginOverlap
  (params (OtherActor :type Actor%20Object%20Reference)))

(event EventTick
  (params (DeltaSeconds :type Float%20%28single-precision%29)))

(fn ConstructionScript)